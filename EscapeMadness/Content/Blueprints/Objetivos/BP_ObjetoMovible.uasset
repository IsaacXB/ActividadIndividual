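; BP_ObjetoMovible is a cube that the player character can push.
; Overlap volumes on the X and Y axes turn on the cube's physics simulation and the character's EmpujarObjeto flag on entry, and turn both off on exit.
; The construction script applies a dynamic material instance, switching to a different material when EsObjetoGanador marks it as the winning object.
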(event `self.ColisionY.OnComponentBeginOverlap`
  (params (OverlappedComponent :type "PrimitiveComponent Object Reference") (OtherActor :type "Actor Object Reference") (OtherComp :type "PrimitiveComponent Object Reference") (OtherBodyIndex :type Integer) (bFromSweep :type Boolean) (SweepResult :type "HitResult Structure (by ref)"))
  ;[1 1 1] Overlap en Y - Activar/Desactivar físicas
  (bind _asbp_personaje (cast `/Game/Personaje/BP_Personaje` OtherActor))
  (`PrimitiveComponent.SetSimulatePhysics` (`self.CuboMovible`) true)
  (set `/Game/Personaje/BP_Personaje.EmpujarObjeto` true _asbp_personaje))

(event `self.ColisionY.OnComponentEndOverlap`
  (params (OverlappedComponent :type "PrimitiveComponent Object Reference") (OtherActor :type "Actor Object Reference") (OtherComp :type "PrimitiveComponent Object Reference") (OtherBodyIndex :type Integer))
  ;[1 1 1] Overlap en Y - Activar/Desactivar físicas
  (bind _asbp_personaje (cast `/Game/Personaje/BP_Personaje` OtherActor))
  (`PrimitiveComponent.SetSimulatePhysics` (`self.CuboMovible`) false)
  (set `/Game/Personaje/BP_Personaje.EmpujarObjeto` false _asbp_personaje))

(event `self.ColisionX.OnComponentBeginOverlap`
  (params (OverlappedComponent :type "PrimitiveComponent Object Reference") (OtherActor :type "Actor Object Reference") (OtherComp :type "PrimitiveComponent Object Reference") (OtherBodyIndex :type Integer) (bFromSweep :type Boolean) (SweepResult :type "HitResult Structure (by ref)"))
  ;[1 1 1] Overlap en X - Activar/Desactivar físicas
  (bind _asbp_personaje (cast `/Game/Personaje/BP_Personaje` OtherActor))
  (`PrimitiveComponent.SetSimulatePhysics` (`self.CuboMovible`) true)
  (set `/Game/Personaje/BP_Personaje.EmpujarObjeto` true _asbp_personaje))

(event `self.ColisionX.OnComponentEndOverlap`
  (params (OverlappedComponent :type "PrimitiveComponent Object Reference") (OtherActor :type "Actor Object Reference") (OtherComp :type "PrimitiveComponent Object Reference") (OtherBodyIndex :type Integer))
  ;[1 1 1] Overlap en X - Activar/Desactivar físicas
  (bind _asbp_personaje (cast `/Game/Personaje/BP_Personaje` OtherActor))
  (`PrimitiveComponent.SetSimulatePhysics` (`self.CuboMovible`) false)
  (set `/Game/Personaje/BP_Personaje.EmpujarObjeto` false _asbp_personaje))

(fn `UserConstructionScript`
  (bind _cubomovible (`self.CuboMovible`))
  (bind _returnvalue (`PrimitiveComponent.CreateDynamicMaterialInstance` _cubomovible 0 "/Engine/VREditor/BasicMeshes/MI_Cube_03.MI_Cube_03" "None"))
  (`PrimitiveComponent.SetMaterial` _cubomovible 0 _returnvalue)
  (if (`self.EsObjetoGanador?`)
    (bind _returnvalue_2 (`PrimitiveComponent.CreateDynamicMaterialInstance` _cubomovible 0 "/Engine/VREditor/BasicMeshes/MI_Cube_02.MI_Cube_02" "None"))
    (`PrimitiveComponent.SetMaterial` _cubomovible 0 _returnvalue_2)))