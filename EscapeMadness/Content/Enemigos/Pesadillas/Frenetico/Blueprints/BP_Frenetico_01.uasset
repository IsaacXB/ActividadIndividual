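; BP_Frenetico_01 is a nightmare enemy that patrols through BT_MovimientoEnemigo and kills the player on contact.
; PawnSensing raises its speed and sends it after BP_Personaje with AIMoveTo.
; A 1500-unit check between player character and PlayerController (not the enemy) gates a one-second attack animation with movement disabled.
; A one-shot capsule hit on the player disables input, shows the death screen and plays a sound.
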(event `self.ReceiveBeginPlay`
  ;[1 1 1] Patrullaje
  (set `CharacterMovementComponent.MaxWalkSpeed` 250.0 (`self.CharacterMovement`))
  (`AIController.RunBehaviorTree` (`AIBlueprintHelperLibrary.GetAIController` self) "/Game/Enemigos/AI/BT_MovimientoEnemigo.BT_MovimientoEnemigo"))

(event `self.PawnSensing.OnSeePawn`
  (params (Pawn :type "Pawn Object Reference"))
  (bind _charactermovement (`self.CharacterMovement`))
  ;[1 1 1] Persecusión
  (set `CharacterMovementComponent.MaxWalkSpeed` 450.0 (`self.CharacterMovement`))
  (bind _asbp_personaje (cast `/Game/Personaje/BP_Personaje` Pawn))
  (`|AIMoveTo` self (`SceneComponent.K2_GetComponentLocation` (`Character.Mesh` _asbp_personaje)) _asbp_personaje
    (:`then`
      _)
    (:`OnSuccess`
      _))
  (if (<= (`self.GetDistanceTo` _asbp_personaje (`GameplayStatics.GetPlayerController` 0)) 1500.0)
    (bind _asbp_anim_frenetico (cast `/Game/Enemigos/Pesadillas/Frenetico/Blueprints/BP_Anim_Frenetico` (`SkeletalMeshComponent.GetAnimInstance` (`self.Mesh`))))
    (set `/Game/Enemigos/Pesadillas/Frenetico/Blueprints/BP_Anim_Frenetico.Atacando` true _asbp_anim_frenetico)
    (`CharacterMovementComponent.DisableMovement` _charactermovement)
    (`KismetSystemLibrary.Delay` 1.0)
    (set `/Game/Enemigos/Pesadillas/Frenetico/Blueprints/BP_Anim_Frenetico.Atacando` false _asbp_anim_frenetico)
    (`CharacterMovementComponent.SetMovementMode` _charactermovement "MOVE_Walking" 0)))

(event `self.CapsuleComponent.OnComponentHit`
  (params (HitComponent :type "PrimitiveComponent Object Reference") (OtherActor :type "Actor Object Reference") (OtherComp :type "PrimitiveComponent Object Reference") (NormalImpulse :type "Vector Structure") (Hit :type "HitResult Structure (by ref)"))
  (cast `/Game/Personaje/BP_Personaje` OtherActor)
  (`/Engine/EditorBlueprintResources/StandardMacros.DoOnce` false
    (:`Completed`
      (`self.DisableInput` (`GameplayStatics.GetPlayerController` 0) null)
      (bind _returnvalue (`|CreateWidget` "/Game/Blueprints/UI/WBP_Pantalla_Muerte.WBP_Pantalla_Muerte_C"))
      (`UserWidget.AddToViewport` _returnvalue 0)
      (`GameplayStatics.PlaySound2D` "/Game/Audio/Muerte/SW_Muerte_Picos.SW_Muerte_Picos" 0.6 1.0 0.0 null null))))

(fn `UserConstructionScript`)