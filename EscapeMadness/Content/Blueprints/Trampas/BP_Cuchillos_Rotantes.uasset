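; Moving blade trap that slides a knife platform back and forth between two points and kills the player on contact.
; On BeginPlay the platform snaps to the start point, then MoveComponentTo, a pause and a FlipFlop form an endless ping-pong loop with configurable timing and easing.
; Overlap of the damage collision with BP_Personaje disables input, shows the death screen and plays a death sound, guarded by DoOnce.
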(event `self.ReceiveBeginPlay`
  (bind _facilidad (`self.Facilidad`))
  (bind _facilidad_2 (`self.Facilidad`))
  (bind _relativelocation (`SceneComponent.RelativeLocation` (`self.PuntoInicial`)))
  (bind _relativelocation_2 (`SceneComponent.RelativeLocation` (`self.PuntoFinal`)))
  ;[1 1 1] Movimiento Plataforma
  (`SceneComponent.K2_SetWorldLocation` (`self.PlataformaCuchillos`) (`SceneComponent.K2_GetComponentLocation` (`self.PuntoInicial`)) false false)
  (`KismetSystemLibrary.MoveComponentTo` (`self.PlataformaCuchillos`) (+ _relativelocation_2 (`KismetMathLibrary.Conv_DoubleToVector` (- (.y _relativelocation_2) 35.0))) (struct) _facilidad_2 _facilidad_2 (`self.TiempoMovimiento`) :!label _label)
  (`KismetSystemLibrary.Delay` (`self.TiempoPausa`) :!label _label_2)
  (`/Engine/EditorBlueprintResources/StandardMacros.FlipFlop`
    (:`A`
      (`KismetSystemLibrary.MoveComponentTo` (`self.PlataformaCuchillos`) (+ _relativelocation (`KismetMathLibrary.Conv_DoubleToVector` (- (.y _relativelocation) 35.0))) (struct) _facilidad _facilidad (`self.TiempoMovimiento`))
      (goto _label_2))
    (:`B`
      (goto _label))))

(event `self.damag collision.OnComponentBeginOverlap`
  (params (OverlappedComponent :type "PrimitiveComponent Object Reference") (OtherActor :type "Actor Object Reference") (OtherComp :type "PrimitiveComponent Object Reference") (OtherBodyIndex :type Integer) (bFromSweep :type Boolean) (SweepResult :type "HitResult Structure (by ref)"))
  ;[1 1 1] Provocar daño
  (bind _asbp_personaje (cast `/Game/Personaje/BP_Personaje` OtherActor))
  (`/Engine/EditorBlueprintResources/StandardMacros.DoOnce` false
    (:`Completed`
      (`self.DisableInput` (`GameplayStatics.GetPlayerController` 0) null)
      (`self.DisableInput` _asbp_personaje null)
      (bind _returnvalue (`|CreateWidget` "/Game/Blueprints/UI/WBP_Pantalla_Muerte.WBP_Pantalla_Muerte_C"))
      (`UserWidget.AddToViewport` _returnvalue 0)
      (`GameplayStatics.PlaySound2D` "/Game/Audio/Muerte/SW_Muerte_Picos.SW_Muerte_Picos" 0.6 1.0 0.0 null null))))

(fn `UserConstructionScript`)