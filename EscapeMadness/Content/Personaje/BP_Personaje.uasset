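; Player character Blueprint with camera-relative movement, mouse look, jumping and crouching.
; Input events drive movement, set button-state flags and adjust jump velocity or crouch acceleration and custom-mode speed, while BeginPlay clamps camera pitch.
; Landing plays one of two random pitch-varied sounds.
; The construction script slaves modular body pieces (torso, pants, shoes, hair, bulge) to the main mesh through master pose.
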(event `self.OnLanded`
  (params (Hit :type "HitResult Structure (by ref)"))
  (bind _returnvalue (`KismetMathLibrary.RandomFloatInRange` 0.7 1.3))
  (switch `int` (`KismetMathLibrary.RandomInteger` 2)
    (:`0`
      (`GameplayStatics.PlaySoundAtLocation` "/Game/Audio/Pasos/SW_Caer1.SW_Caer1" (0.0 0.0 0.0) (struct) 0.1 _returnvalue 0.0 null null null))
    (:`1`
      (`GameplayStatics.PlaySoundAtLocation` "/Game/Audio/Pasos/SW_Caer2.SW_Caer2" (0.0 0.0 0.0) (struct) 0.1 _returnvalue 0.0 null null null))))

(event `self.ReceiveBeginPlay`
  (bind _returnvalue (`GameplayStatics.GetPlayerCameraManager` 0))
  ;[1 1 1] Camera Min/Max Pitch
  (set `PlayerCameraManager.ViewPitchMax` 20.0 _returnvalue)
  (set `PlayerCameraManager.ViewPitchMin` -5.0 _returnvalue))

(event `InputAxis|Mover Arriba`
  (params (AxisValue :type "Float (single-precision)"))
  ;[1 1 1] Movimiento Personaje
  (`self.AddMovementInput` (`KismetMathLibrary.GetForwardVector` (`KismetMathLibrary.MakeRotator` 0.0 0.0 (.yaw (`self.GetControlRotation`)))) AxisValue))

(event `InputAxis|Mover Derecha`
  (params (AxisValue :type "Float (single-precision)"))
  ;[1 1 1] Movimiento Personaje
  (`self.AddMovementInput` (`KismetMathLibrary.GetRightVector` (`KismetMathLibrary.MakeRotator` 0.0 0.0 (.yaw (`self.GetControlRotation`)))) AxisValue))

(event `InputAxis|Mouse X`
  (params (AxisValue :type "Float (single-precision)"))
  ;[1 1 1] Mira del Mouse
  (`self.AddControllerYawInput` AxisValue))

(event `InputAxis|Mouse Y`
  (params (AxisValue :type "Float (single-precision)"))
  ;[1 1 1] Mira del Mouse
  (`self.AddControllerPitchInput` AxisValue))

(event `InputAction|Saltar`
  (params (Key :type "Key Structure"))
  ;[1 1 1] Saltar
  (:`Pressed`
    (set `self.Botón Saltar presionado` (`self.CanJump`))
    (`self.Jump`)
    (bind _ascharacter_movement_component (cast `CharacterMovementComponent` (`self.GetMovementComponent`)))
    (if (> (`KismetMathLibrary.VSize` (`MovementComponent.Velocity` _ascharacter_movement_component)) 0.0)
      (set `CharacterMovementComponent.JumpZVelocity` 500.0 _ascharacter_movement_component)
      (else
        (set `CharacterMovementComponent.JumpZVelocity` 500.0 _ascharacter_movement_component))))
  (:`Released`
    (set `self.Botón Saltar presionado` false)
    (`self.StopJumping`)))

(event `InputAction|Agacharse`
  (params (Key :type "Key Structure"))
  (bind _charactermovement (`self.CharacterMovement`))
  ;[1 1 1] Agacharse
  (:`Pressed`
    (set `self.Botón agacharse presionado` true)
    (`self.Crouch`)
    (set `CharacterMovementComponent.MaxAcceleration` 100.0 _charactermovement)
    (set `CharacterMovementComponent.MaxCustomMovementSpeed` 75.0 _charactermovement))
  (:`Released`
    (set `self.Botón agacharse presionado` false)
    (`self.UnCrouch`)
    (set `CharacterMovementComponent.MaxAcceleration` 300.0 _charactermovement)
    (set `CharacterMovementComponent.MaxCustomMovementSpeed` 300.0 _charactermovement)))

(fn `UserConstructionScript`
  (`SkinnedMeshComponent.SetLeaderPoseComponent` (`self.Torso`) (`self.Mesh`) false)
  (`SkinnedMeshComponent.SetLeaderPoseComponent` (`self.Pantalones`) (`self.Mesh`) false)
  (`SkinnedMeshComponent.SetLeaderPoseComponent` (`self.Zapatos`) (`self.Mesh`) false)
  (`SkinnedMeshComponent.SetLeaderPoseComponent` (`self.Pelo`) (`self.Mesh`) false)
  (`SkinnedMeshComponent.SetLeaderPoseComponent` (`self.Bulto`) (`self.Mesh`) false))