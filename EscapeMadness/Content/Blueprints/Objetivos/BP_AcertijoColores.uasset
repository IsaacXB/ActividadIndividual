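; Colour-sequence puzzle actor that opens a referenced door when four colours are entered in the right order.
; On BeginPlay it paints four solution meshes with the configured code, using bright dynamic material instances.
; ActualizarCodigo checks each submitted colour against the current step, lighting its progress mesh, or resetting all progress on a mistake.
; The final match sets the door open, turns it green and activates an objective sound.
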(event `self.ReceiveBeginPlay`
  (`self.Asignar Solucion`))

(fn `Actualizar Codigo`
  (params (Color :type "/Game/Blueprints/Enumeradores/Enum_Colores Enum" :default "NewEnumerator0"))
  (returns (`EsCodigoCorrecto?` :type Boolean))
  (bind _puerta_referencia (`self.Puerta_Referencia`))
  (switch `int` (`self.Codigo`)
    (:`0`
      (if (`|EnumEquality` Color (`self.CodigoSolucion1`))
        (`self.Asignar Color Solucion` Color (`self.Color1`))
        (`/Engine/EditorBlueprintResources/StandardMacros.IncrementInt` (`self.Codigo`)
          (:`  `
            (return true)))
        (else
          _)))
    (:`1`
      (if (`|EnumEquality` Color (`self.CodigoSolucion2`))
        (`self.Asignar Color Solucion` Color (`self.Color2`))
        (`/Engine/EditorBlueprintResources/StandardMacros.IncrementInt` (`self.Codigo`)
          (:`  `
            (return true)))
        (else
          _)))
    (:`2`
      (if (`|EnumEquality` Color (`self.CodigoSolucion3`))
        (`self.Asignar Color Solucion` Color (`self.Color3`))
        (`/Engine/EditorBlueprintResources/StandardMacros.IncrementInt` (`self.Codigo`)
          (:`  `
            (return true)))
        (else
          _)))
    (:`3`
      (if (`|EnumEquality` Color (`self.CodigoSolucion4`))
        (`self.Asignar Color Solucion` Color (`self.Color4`))
        (set `/Game/Blueprints/Puertas/BP_Puerta_Salida.Abierto?` true _puerta_referencia)
        (`ActorComponent.Activate` (`self.SonidoObjetivo`) false)
        (`PrimitiveComponent.SetMaterial` (`/Game/Blueprints/Puertas/BP_Puerta_Salida.Puerta` _puerta_referencia) 0 "/Game/Materiales/M_Verde_Brillante.M_Verde_Brillante")
        (return true)
        (else
          _))))
  (`self.Desasignar Codigo`)
  (return false))

(fn `Asignar Color Solucion`
  (params (Color :type "/Game/Blueprints/Enumeradores/Enum_Colores Enum" :default "NewEnumerator0") (Target :type "PrimitiveComponent Object Reference"))
  (switch `/Game/Blueprints/Enumeradores/Enum_Colores` Color
    (:`NewEnumerator0`
      (bind _returnvalue (`PrimitiveComponent.CreateDynamicMaterialInstance` Target 0 "/Game/Materiales/M_Rojo_Brillante.M_Rojo_Brillante" "None"))
      (`PrimitiveComponent.SetMaterial` Target 0 _returnvalue))
    (:`NewEnumerator1`
      (bind _returnvalue_2 (`PrimitiveComponent.CreateDynamicMaterialInstance` Target 0 "/Game/Materiales/M_Azul_Brillante.M_Azul_Brillante" "None"))
      (`PrimitiveComponent.SetMaterial` Target 0 _returnvalue_2))
    (:`NewEnumerator2`
      (bind _returnvalue_3 (`PrimitiveComponent.CreateDynamicMaterialInstance` Target 0 "/Game/Materiales/M_Verde_Brillante.M_Verde_Brillante" "None"))
      (`PrimitiveComponent.SetMaterial` Target 0 _returnvalue_3))
    (:`NewEnumerator3`
      (bind _returnvalue_4 (`PrimitiveComponent.CreateDynamicMaterialInstance` Target 0 "/Game/Materiales/M_Marron_Brillante.M_Marron_Brillante" "None"))
      (`PrimitiveComponent.SetMaterial` Target 0 _returnvalue_4))
    (:`NewEnumerator4`
      (bind _returnvalue_5 (`PrimitiveComponent.CreateDynamicMaterialInstance` Target 0 "/Engine/BasicShapes/BasicShapeMaterial.BasicShapeMaterial" "None"))
      (`PrimitiveComponent.SetMaterial` Target 0 _returnvalue_5))))

(fn `Asignar Solucion`
  (`self.Asignar Color Solucion` (`self.CodigoSolucion1`) (`self.Solucion1`))
  (`self.Asignar Color Solucion` (`self.CodigoSolucion2`) (`self.Solucion2`))
  (`self.Asignar Color Solucion` (`self.CodigoSolucion3`) (`self.Solucion3`))
  (`self.Asignar Color Solucion` (`self.CodigoSolucion4`) (`self.Solucion4`)))

(fn `Desasignar Codigo`
  (`self.Asignar Color Solucion` "NewEnumerator4" (`self.Color1`))
  (`self.Asignar Color Solucion` "NewEnumerator4" (`self.Color2`))
  (`self.Asignar Color Solucion` "NewEnumerator4" (`self.Color3`))
  (`self.Asignar Color Solucion` "NewEnumerator4" (`self.Color4`))
  (set `self.Codigo` 0))

(fn `UserConstructionScript`)