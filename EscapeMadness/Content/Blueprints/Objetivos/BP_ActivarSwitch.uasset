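; BP_ActivarSwitch is a colored switch that submits its color to a referenced code puzzle when the player character touches it.
; On BeginPlay it sets the plane to a bright dynamic material matching its ColorSwitch value (red, blue, green or brown).
; Overlapping its collision box with BP_Personaje passes the color to AcertijoReferencia's ActualizarCodigo, whose boolean result activates the success or failure sound.
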(event `self.ReceiveBeginPlay`
  (bind _plane (`self.Plane`))
  (switch `/Game/Blueprints/Enumeradores/Enum_Colores` (`self.ColorSwitch`)
    (:`NewEnumerator0`
      (bind _returnvalue (`PrimitiveComponent.CreateDynamicMaterialInstance` _plane 0 "/Game/Materiales/M_Rojo_Brillante.M_Rojo_Brillante" "None"))
      (`PrimitiveComponent.SetMaterial` _plane 0 _returnvalue))
    (:`NewEnumerator1`
      (bind _returnvalue_2 (`PrimitiveComponent.CreateDynamicMaterialInstance` _plane 0 "/Game/Materiales/M_Azul_Brillante.M_Azul_Brillante" "None"))
      (`PrimitiveComponent.SetMaterial` _plane 0 _returnvalue_2))
    (:`NewEnumerator2`
      (bind _returnvalue_3 (`PrimitiveComponent.CreateDynamicMaterialInstance` _plane 0 "/Game/Materiales/M_Verde_Brillante.M_Verde_Brillante" "None"))
      (`PrimitiveComponent.SetMaterial` _plane 0 _returnvalue_3))
    (:`NewEnumerator3`
      (bind _returnvalue_4 (`PrimitiveComponent.CreateDynamicMaterialInstance` _plane 0 "/Game/Materiales/M_Marron_Brillante.M_Marron_Brillante" "None"))
      (`PrimitiveComponent.SetMaterial` _plane 0 _returnvalue_4))))

(event `self.CajaDeColision.OnComponentBeginOverlap`
  (params (OverlappedComponent :type "PrimitiveComponent Object Reference") (OtherActor :type "Actor Object Reference") (OtherComp :type "PrimitiveComponent Object Reference") (OtherBodyIndex :type Integer) (bFromSweep :type Boolean) (SweepResult :type "HitResult Structure (by ref)"))
  (cast `/Game/Personaje/BP_Personaje` OtherActor)
  (bind _escodigocorrecto_ (`/Game/Blueprints/Objetivos/BP_AcertijoColores.Actualizar Codigo` (`self.Acertijo_Referencia`) (`self.ColorSwitch`)))
  (if _escodigocorrecto_
    (`ActorComponent.Activate` (`self.SonidoObjetivoExitoso`) false)
    (else
      (`ActorComponent.Activate` (`self.SonidoObjetivoFallido`) false))))

(fn `UserConstructionScript`)