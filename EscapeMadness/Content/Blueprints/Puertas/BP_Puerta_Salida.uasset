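; BP_Puerta_Salida is an exit door that moves the player to the MapaPruebas level.
; When a BP_Personaje overlaps its collision box while the Abierto flag is true, a DoOnce gate triggers the transition a single time.
; It adds a WBP_Efecto_Desvanecer widget to the viewport, plays its fade animation, then opens the hardcoded level after a short delay.
; Nothing in this Blueprint sets Abierto.
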(event `self.Caja de colision.OnComponentBeginOverlap`
  (params (OverlappedComponent :type "PrimitiveComponent Object Reference") (OtherActor :type "Actor Object Reference") (OtherComp :type "PrimitiveComponent Object Reference") (OtherBodyIndex :type Integer) (bFromSweep :type Boolean) (SweepResult :type "HitResult Structure (by ref)"))
  ;[1 1 1] Abrir Puerta
  (cast `/Game/Personaje/BP_Personaje` OtherActor)
  (if (`self.Abierto?`)
    (`/Engine/EditorBlueprintResources/StandardMacros.DoOnce` false
      (:`Completed`
        (bind _returnvalue (`|CreateWidget` "/Game/Blueprints/UI/WBP_Efecto_Desvanecer.WBP_Efecto_Desvanecer_C"))
        (`UserWidget.AddToViewport` _returnvalue 0)
        (`UserWidget.PlayAnimation` _returnvalue (`/Game/Blueprints/UI/WBP_Efecto_Desvanecer.Desvanecer` _returnvalue) 0.0 1 "Forward" 1.0 false)
        (`KismetSystemLibrary.Delay` 0.25)
        (`GameplayStatics.OpenLevel` (`self.Mapa_Pruebas`))))))

(fn `UserConstructionScript`)