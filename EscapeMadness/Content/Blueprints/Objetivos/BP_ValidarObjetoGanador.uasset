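; BP_ValidarObjetoGanador is a goal zone that opens a linked door when the winning movable object enters it.
; A collision box overlap checks for a BP_ObjetoMovible flagged EsObjetoGanador, turns the red Meta mesh green and activates a sound.
; After a short delay it paints PuertaReferencia's door green and sets it open.
; Leaving the zone only turns Meta red again; the door stays open.
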(event `self.ReceiveBeginPlay`
  (bind _meta (`self.Meta`))
  (bind _returnvalue (`PrimitiveComponent.CreateDynamicMaterialInstance` _meta 0 "/Game/Materiales/M_Rojo_Brillante.M_Rojo_Brillante" "None"))
  (`PrimitiveComponent.SetMaterial` _meta 0 _returnvalue))

(event `self.CajaDeColision.OnComponentBeginOverlap`
  (params (OverlappedComponent :type "PrimitiveComponent Object Reference") (OtherActor :type "Actor Object Reference") (OtherComp :type "PrimitiveComponent Object Reference") (OtherBodyIndex :type Integer) (bFromSweep :type Boolean) (SweepResult :type "HitResult Structure (by ref)"))
  (bind _puerta_referencia (`self.Puerta_Referencia`))
  (bind _meta (`self.Meta`))
  ;[1 1 1] Si es el objeto ganador => cambiar color a verde
  (bind _asbp_objeto_movible (cast `/Game/Blueprints/Objetivos/BP_ObjetoMovible` OtherActor))
  (if (`/Game/Blueprints/Objetivos/BP_ObjetoMovible.EsObjetoGanador?` _asbp_objeto_movible)
    (bind _returnvalue (`PrimitiveComponent.CreateDynamicMaterialInstance` _meta 0 "/Game/Materiales/M_Verde_Brillante.M_Verde_Brillante" "None"))
    (`PrimitiveComponent.SetMaterial` _meta 0 _returnvalue)
    (`ActorComponent.Activate` (`self.SonidoObjetivo`) false)
    (`KismetSystemLibrary.Delay` 0.6)
    (`PrimitiveComponent.SetMaterial` (`/Game/Blueprints/Puertas/BP_Puerta_Salida.Puerta` _puerta_referencia) 0 "/Game/Materiales/M_Verde_Brillante.M_Verde_Brillante")
    (set `/Game/Blueprints/Puertas/BP_Puerta_Salida.Abierto?` true _puerta_referencia)))

(event `self.CajaDeColision.OnComponentEndOverlap`
  (params (OverlappedComponent :type "PrimitiveComponent Object Reference") (OtherActor :type "Actor Object Reference") (OtherComp :type "PrimitiveComponent Object Reference") (OtherBodyIndex :type Integer))
  (bind _meta (`self.Meta`))
  ;[1 1 1] Si sale del area ganadora => cambiar a color rojo
  (bind _asbp_objeto_movible (cast `/Game/Blueprints/Objetivos/BP_ObjetoMovible` OtherActor))
  (if (`/Game/Blueprints/Objetivos/BP_ObjetoMovible.EsObjetoGanador?` _asbp_objeto_movible)
    (bind _returnvalue (`PrimitiveComponent.CreateDynamicMaterialInstance` _meta 0 "/Game/Materiales/M_Rojo_Brillante.M_Rojo_Brillante" "None"))
    (`PrimitiveComponent.SetMaterial` _meta 0 _returnvalue)))

(fn `UserConstructionScript`)