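; Moving platform that shuttles back and forth between two points, starting either active or waiting for activation.
; At BeginPlay it snaps to Punto1, then, if active, loops eased MoveComponentTo moves, alternated by a FlipFlop after each pause.
; An inactive platform glows red with muted movement sound until the ActivarPlataforma dispatcher turns it green, restores the volume and starts the loop.
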(event `self.ReceiveBeginPlay`
  (bind _facilidad (`self.Facilidad`))
  (bind _plataformabrillo (`self.PlataformaBrillo`))
  (bind _facilidad_2 (`self.Facilidad`))
  (add `self.Activar Plataforma` (delegate `Active`))
  (`SceneComponent.K2_SetWorldLocation` (`self.Plataforma`) (`SceneComponent.K2_GetComponentLocation` (`self.Punto 1`)) false false)
  (if (`self.Activate`)
    (`PrimitiveComponent.SetMaterial` _plataformabrillo 0 "/Game/Materiales/M_Verde_Brillante.M_Verde_Brillante")
    (`KismetSystemLibrary.MoveComponentTo` (`self.Plataforma`) (`SceneComponent.RelativeLocation` (`self.Punto 2`)) (struct) _facilidad _facilidad (`self.Tiempo Movimiento`) :!label _label)
    (`KismetSystemLibrary.Delay` (`self.Tiempo Pausa`) :!label _label_2)
    (`/Engine/EditorBlueprintResources/StandardMacros.FlipFlop`
      (:`A`
        (`KismetSystemLibrary.MoveComponentTo` (`self.Plataforma`) (`SceneComponent.RelativeLocation` (`self.Punto 1`)) (struct) _facilidad_2 _facilidad_2 (`self.Tiempo Movimiento`))
        (goto _label_2))
      (:`B`
        (goto _label)))
    (else
      (`PrimitiveComponent.SetMaterial` _plataformabrillo 0 "/Game/Materiales/M_Rojo_Brillante.M_Rojo_Brillante")
      (`AudioComponent.SetVolumeMultiplier` (`self.Plataforma Movimiento`) 0.0))))

(event `Active`
  (`PrimitiveComponent.SetMaterial` (`self.PlataformaBrillo`) 0 "/Game/Materiales/M_Verde_Brillante.M_Verde_Brillante")
  (`AudioComponent.SetVolumeMultiplier` (`self.Plataforma Movimiento`) 1.0)
  (goto _label))

(fn `UserConstructionScript`)